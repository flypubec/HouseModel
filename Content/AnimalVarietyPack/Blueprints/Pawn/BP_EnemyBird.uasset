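; BP_EnemyBird is a bird pawn with flight steering, set up around the DON navigation manager.
; Custom movement input while flying smoothly banks and pitches the bird within clamped limits, then applies speed-scaled movement; when not flying, Tick pushes it downward.
; BeginPlay caches the navigation manager and nav mesh bounds, then briefly randomizes animation rate to desynchronize starting frames.
; The delayed behavior tree startup is unconnected and never runs.
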(event `self.AddMovementInputCustom`
  (params (WorldDirection :type "Vector Structure") (ScaleValue :type "Float (single-precision)"))
  (if (`self.isFlying`)
    (`self.K2_SetActorRotation` (`KismetMathLibrary.RInterpTo` (`self.K2_GetActorRotation`) (`KismetMathLibrary.MakeRotator` (`KismetMathLibrary.FClamp` (.roll (`KismetMathLibrary.MakeRotFromX` (* (`KismetMathLibrary.MirrorVectorByNormal` (`self.GetVelocity`) WorldDirection) -1))) -30.0 30.0) (`KismetMathLibrary.FClamp` (.pitch (`KismetMathLibrary.MakeRotFromX` (* (`KismetMathLibrary.MirrorVectorByNormal` (`self.GetVelocity`) WorldDirection) -1))) -30.0 30.0) (.yaw (`KismetMathLibrary.MakeRotFromX` (* (`KismetMathLibrary.MirrorVectorByNormal` (`self.GetVelocity`) WorldDirection) -1)))) (`GameplayStatics.GetWorldDeltaSeconds`) 5.0))
    (`self.AddMovementInput` WorldDirection (* ScaleValue (`self.Bot Speed Scale`)))))

(event `self.ReceiveTick`
  (params (DeltaSeconds :type "Float (single-precision)"))
  (if (not (`self.isFlying`))
    (`self.AddMovementInput` (0.0 0.0 -1.0))))

(event `self.ReceiveBeginPlay`
  (bind _skeletalcomponent (`self.SkeletalComponent`))
  (set `self.DON_NavigationManager` (`DonNavigationHelper.DonNavigationManager`))
  (bind _outactors (`GameplayStatics.GetAllActorsOfClass` "/Script/NavigationSystem.NavMeshBoundsVolume"))
  (set `self.NavMeshBounds` (`|GetArrayItem` _outactors))
  (set `SkeletalMeshComponent.GlobalAnimRateScale` (`KismetMathLibrary.RandomFloatInRange` 10.0 500.0) _skeletalcomponent)
  (`KismetSystemLibrary.Delay` 0.2)
  (set `SkeletalMeshComponent.GlobalAnimRateScale` 1.0 _skeletalcomponent))

(fn `UserConstructionScript`)